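; BP_Enemy_Test is a test enemy Blueprint that takes damage and switches to physics simulation when its health runs out.
; AnyDamage subtracts the truncated damage from CurrentHealth, then sets physics simulation on the Mesh according to whether health is at or below zero.
; BeginPlay, overlap and Tick are disabled placeholder events, and the construction script only calls its parent.
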(event EventBeginPlay
  (|CallParentFunction) ; Este nó está desativado e não será chamado.\nArraste os pinos para criar funcionalidade.
)

(event Collision|EventActorBeginOverlap
  (params (OtherActor :type Actor%20Object%20Reference))
  (|CallParentFunction OtherActor) ; Este nó está desativado e não será chamado.\nArraste os pinos para criar funcionalidade.
)

(event EventTick
  (params (DeltaSeconds :type Float%20%28single-precision%29))
  (|CallParentFunction DeltaSeconds) ; Este nó está desativado e não será chamado.\nArraste os pinos para criar funcionalidade.
)

(event Game|Damage|EventAnyDamage
  (params (Damage :type Float%20%28single-precision%29) (DamageType :type Damage%20Type%20Object%20Reference) (InstigatedBy :type Controller%20Object%20Reference) (DamageCauser :type Actor%20Object%20Reference))
  (bind _output_get (Variables|Default|SetCurrent%20Health (- (Variables|Default|GetCurrent%20Health) (Math|Float|Truncate Damage))))
  (Physics|SetSimulatePhysics (Variables|Character|GetMesh) (<= _output_get 0)))

(fn ConstructionScript
  (|CallParentFunction))