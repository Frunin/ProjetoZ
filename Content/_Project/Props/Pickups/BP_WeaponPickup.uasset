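; BP_WeaponPickup is a weapon pickup prop that gives a character a weapon when interacted with.
; Its Interact event calls SpawnWeapon on the interacting character, passing the pickup's WeaponToSpawn and its own location, then destroys the pickup.
; BeginPlay, overlap and Tick are disabled stubs, so all of its own logic runs from Interact.
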(event EventBeginPlay
  (|CallParentFunction) ; Este nó está desativado e não será chamado.\nArraste os pinos para criar funcionalidade.
)

(event Collision|EventActorBeginOverlap
  (params (OtherActor :type Actor%20Object%20Reference))
  (|CallParentFunction OtherActor) ; Este nó está desativado e não será chamado.\nArraste os pinos para criar funcionalidade.
)

(event EventTick
  (params (DeltaSeconds :type Float%20%28single-precision%29))
  (|CallParentFunction DeltaSeconds) ; Este nó está desativado e não será chamado.\nArraste os pinos para criar funcionalidade.
)

(event EventInteract
  (params (Char%20Picking%20Up :type BP%20Third%20Person%20Character%20Object%20Reference))
  (Default|SpawnWeapon Char%20Picking%20Up (Variables|Default|GetWeaponToSpawn) (Transformation|GetActorLocation))
  (Actor|DestroyActor))

(fn ConstructionScript
  (|CallParentFunction))